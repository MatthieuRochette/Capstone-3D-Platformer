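; Static excavator prop whose light states and body color are applied in the construction script.
; A dynamic instance of the cabin material takes the headlight, brake, reverse, turn signal and engine booleans as 0/1 scalar parameters that drive masked emissive lighting.
; FCreateBodyMatInst then replaces each slot using the body material with a dynamic instance and tints it with the excavator color.
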(fn ConstructionScript
  ;[1 1 1] Create material instance for lights
  (bind _returnvalue (Rendering|Material|CreateDynamicMaterialInstance (Variables|Default|GetStaticMesh) 3 "/Game/PB_Excavator/BP_Excavator/Materials/MI_Cabin_Inst.MI_Cabin_Inst" "None" :!class /Script/Engine.PrimitiveComponent))
  (Variables|Default|SetLightMatInstance _returnvalue)
  ;[1 1 1] Lights are based on textures that are inside the material (see the cabin material to check how this works). Basically a scalar parameter is set inside the material and will use a mask for that light to use the emissive output of the material
  ;;[1 1 1] Headlights on or off
  (Rendering|Material|SetScalarParameterValue (Variables|Default|GetLightMatInstance) "Headlights?" (Math|Float|SelectFloat 1.0 0.0 (Variables|Default|GetHeadLightsOn)) :!class /Script/Engine.MaterialInstanceDynamic)
  ;;[1 1 1] Brake lights on or off
  (Rendering|Material|SetScalarParameterValue (Variables|Default|GetLightMatInstance) "StopLights?" (Math|Float|SelectFloat 1.0 0.0 (Variables|Default|GetIsBraking)) :!class /Script/Engine.MaterialInstanceDynamic)
  ;;[1 1 1] Reverse light on or off
  (Rendering|Material|SetScalarParameterValue (Variables|Default|GetLightMatInstance) "RearLights?" (Math|Float|SelectFloat 1.0 0.0 (Variables|Default|GetIsReverse)) :!class /Script/Engine.MaterialInstanceDynamic)
  ;;[1 1 1] Turning Light
  (Rendering|Material|SetScalarParameterValue (Variables|Default|GetLightMatInstance) "ArrowL" (Math|Float|SelectFloat 1.0 0.0 (Variables|Default|GetIsTurningL)) :!class /Script/Engine.MaterialInstanceDynamic)
  ;;[1 1 1] Turn r light on or off
  (Rendering|Material|SetScalarParameterValue (Variables|Default|GetLightMatInstance) "ArrowR" (Math|Float|SelectFloat 1.0 0.0 (Variables|Default|GetIsTurningR)) :!class /Script/Engine.MaterialInstanceDynamic)
  ;;[1 1 1] Turn r light on or off
  (Rendering|Material|SetScalarParameterValue (Variables|Default|GetLightMatInstance) "EngineOn" (Math|Float|SelectFloat 1.0 0.0 (Variables|Default|GetEngineStarted)) :!class /Script/Engine.MaterialInstanceDynamic)
  (CallFunction|FCreateBodyMatInst))

(fn FCreateBodyMatInst
  (bind _bodymaterialinstances (Variables|Default|GetBodyMaterialInstances))
  (Utilities|Array|Clear _bodymaterialinstances)
  (Utilities|Array|Resize _bodymaterialinstances 0)
  (for (_array_element _array_index) (Rendering|Material|GetMaterials (Variables|Default|GetStaticMesh))
    (if (== _array_element "/Game/PB_Excavator/BP_Excavator/Materials/Mi_Corpus_Inst.Mi_Corpus_Inst")
      (bind _returnvalue (Rendering|Material|CreateDynamicMaterialInstance (Variables|Default|GetStaticMesh) _array_index _array_element "None" :!class /Script/Engine.PrimitiveComponent))
      (Utilities|Array|Add (Variables|Default|GetBodyMaterialInstances) _returnvalue)))
  (for _array_element_2 (Variables|Default|GetBodyMaterialInstances)
    (Rendering|Material|SetVectorParameterValue _array_element_2 "Color" (Variables|Default|GetExcatorColor) :!class /Script/Engine.MaterialInstanceDynamic)))