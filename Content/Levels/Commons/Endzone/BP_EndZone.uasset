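; BP_EndZone is a level-end trigger that celebrates on overlap and loads the next level.
; Each actor overlap spawns two spark emitters and a flamethrower emitter at the zone and plays a firework sound.
; A DoOnce then waits briefly and opens the level found in LevelsDict by NextLevel.
; After that open call, it sets EngineStarted false if the overlapping actor is a BP_Excavator.
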(event EventBeginPlay)

(event Collision|EventActorBeginOverlap
  (params (OtherActor :type Actor%20Object%20Reference))
  (bind _returnvalue (Transformation|GetActorLocation))
  (Utilities|FlowControl|Sequence
    (:then_0
      (Effects|SpawnEmitteratLocation "/Game/Levels/Commons/Endzone/P_Sparks_D_Copy.P_Sparks_D_Copy" _returnvalue))
    (:then_1
      (Effects|SpawnEmitteratLocation "/Game/Levels/Commons/Endzone/P_Sparks_G_Cpoy.P_Sparks_G_Cpoy" _returnvalue))
    (:then_2
      (Effects|SpawnEmitteratLocation "/Game/Levels/Commons/Endzone/P_Flamethrower_Copy.P_Flamethrower_Copy" _returnvalue))
    (:then_3
      (Audio|PlaySoundatLocation "/Game/Levels/Commons/Endzone/S_Firework.S_Firework" _returnvalue "0, 0, 0" 1.0 1.0 0.0 0 0 0))
    (:then_4
      (Utilities|FlowControl|DoOnce false
        (:Completed
          (Utilities|FlowControl|Delay 3.5)
          (Game|OpenLevel(byName) (.Value (Utilities|Map|Find (Variables|Default|GetLevels_Dict) (Variables|Default|GetNext%20level))))
          (bind _asbp_excavator (Utilities|Casting|CastToBP_Excavator OtherActor))
          (Variables|/Game/PB_Excavator/BP_Excavator/Blueprints/BP_Excavator.BP_Excavator_C|SetEngineStarted _asbp_excavator false))))))

(event EventTick
  (params (DeltaSeconds :type Float%20%28single-precision%29)))

(fn ConstructionScript)